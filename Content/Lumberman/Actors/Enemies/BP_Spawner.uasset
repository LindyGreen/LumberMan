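; BP_Spawner is an enemy spawner that scales with dungeon level and opens the level gates once its enemies are killed.
; The dungeon level sets the enemy count and spawn interval, and a looping timer spawns until that count is reached.
; Each enemy receives a spawner reference, and EnemyKilled counts deaths before messaging the level master.
; Both Melee and Ranged types currently select BP_Enemy.
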(event Custom|SpawnAnEnemy
  (bind _returnvalue (Game|SpawnActorfromClass (Utilities|Select :Index (Variables|Default|GetEnemyType) :NewEnumerator0 "/Game/Lumberman/Actors/Enemies/BP_Enemy.BP_Enemy_C" :NewEnumerator1 "/Game/Lumberman/Actors/Enemies/BP_Enemy.BP_Enemy_C") (Transformation|GetActorTransform) "AdjustIfPossibleButAlwaysSpawn" "MultiplyWithRoot" 0 0))
  (Class|BPIInteractable|WhosYourDaddy?(Message) _returnvalue self)
  (bind _result (Math|Integer|IncrementInt (Variables|Default|GetEnemiesSpawned))
    (:%20%20
      (if (== _result (Variables|Default|GetNumberOfEnemiesToSpawn))
        (Utilities|Time|ClearandInvalidateTimerbyHandle (Variables|Default|GetSpawnTimerHandle))))))

(event EventGetDungeonLevel
  (params (DungeonLevel :type Integer))
  (Variables|Default|SetNumberOfEnemiesToSpawn (* DungeonLevel 5))
  (Variables|Default|SetTimeBetweenSpawns (|(3/DungeonLevel) (Math|Conversions|ToFloat(Integer) DungeonLevel)))
  (bind _returnvalue (Utilities|Time|SetTimerbyEvent (delegate Custom|SpawnAnEnemy) (Variables|Default|GetTimeBetweenSpawns) true false 1.0))
  (Variables|Default|SetSpawnTimerHandle _returnvalue))

(event EventEnemyKilled
  (bind _result (Math|Integer|IncrementInt (Variables|Default|GetEnemiesKilled))
    (:%20%20
      (if (== _result (Variables|Default|GetNumberOfEnemiesToSpawn))
        (Class|BPIGauntlet|OpenGates(Message) (Variables|Default|GetLevelMasterRef))))))

(fn ConstructionScript)
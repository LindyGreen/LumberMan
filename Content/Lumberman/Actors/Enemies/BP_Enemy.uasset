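; Zombie enemy character that takes chop hits from the player and attacks back at close range.
; A gate limits hits to about one per second, each lowering HP, updating the HP bar widget, playing a hit reaction and launching it away from the player.
; Knockback scales with the damage value read from the game instance.
; At zero HP it notifies its assigned Daddy object and destroys itself after a short delay.
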(event Custom|TakeDamage
  (bind _knockback_power (Variables|Default|GetKnockback%20Power))
  (bind (_returnvalue_x _returnvalue_y) (|LauinchDirCalc _knockback_power))
  (bind _output_get (Variables|Default|SetHP (- (Variables|Default|GetHP) (stale EventChopChop Damage))))
  (CallFunction|UpdateHPBar)
  (Character|LaunchCharacter self (Math|Vector|MakeVector _returnvalue_x _returnvalue_y 1e+01) false false)
  (Animation|PlayAnimMontage "/Game/Lumberman/Assets/Animations/MeleeZombie/Zombie_HitReact.Zombie_HitReact" 2.0 "None")
  (if (>= 0.0 _output_get)
    (Class|BPIGauntlet|EnemyKilled(Message) (Variables|Default|GetDaddy))
    (Utilities|FlowControl|Delay 1.0)
    (Actor|DestroyActor) ; insert some damage SFX/VFX here
  ))

(event EventBeginPlay
  (bind _asgi (Utilities|Casting|CastToGI (Game|GetGameInstance)))
  (bind _output_get (Variables|Default|SetPlayerDamage (Default|GetDamageVar _asgi)))
  (Variables|Default|SetKnockback%20Power (* _output_get 2e+01)))

(event EventAttack
  (params (AttackTarget :type Actor%20Object%20Reference))
  (Animation|PlayAnimMontage "/Game/Lumberman/Assets/Animations/MeleeZombie/Zombie_attack.Zombie_attack" 2.0 "None")
  (if (< (Transformation|GetDistanceTo (Game|Player|GetPlayerPawn 0)) 1e+02)
    (Class|BPIAttackable|TakeDamage(Message) AttackTarget (Variables|Default|GetEnemyDamage))))

(event EventWhosYourDaddy?
  (params (Daddy :type Actor%20Object%20Reference))
  (Variables|Default|SetDaddy Daddy))

(event EventChopChop
  (params (Damage :type Float%20%28double-precision%29))
  (Utilities|FlowControl|Gate false :!label _label
    (:Exit
      (Utilities|FlowControl|Sequence
        (:then_0
          (CallFunction|TakeDamage)
          (goto _label Close))
        (:then_1
          (Utilities|FlowControl|Delay 1.0)
          (goto _label Open))))))

(fn ConstructionScript
  (Variables|Default|SetHP (Variables|Default|GetMaxHP)))

(fn UpdateHPBar
  (Class|BPIUI|GetHpPercentage(Message) (UserInterface|GetWidget (Variables|Default|GetHP_Bar)) (/ (Variables|Default|GetHP) (Variables|Default|GetMaxHP))))

(fn WhatTypeAreYou
  (return "NewEnumerator2"))
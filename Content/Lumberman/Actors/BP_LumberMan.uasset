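; BP_LumberMan is the playable lumberjack character, with axis movement and an axe attached to its right hand socket.
; A sphere overlap tracks interactable actors; a looping timer toggles hit collision and plays a spin-swing montage while any are present.
; Hit overlaps send ChopChopMessage with a damage value.
; The Game Instance holds player stats, receiving incoming damage and the HP reset at BeginPlay.
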(event OnComponentBeginOverlap(r)
  (params (OverlappedComponent :type Primitive%20Component%20Object%20Reference) (OtherActor :type Actor%20Object%20Reference) (OtherComp :type Primitive%20Component%20Object%20Reference) (OtherBodyIndex :type Integer) (bFromSweep :type Boolean) (SweepResult :type Hit%20Result%20Structure%20%28by%20ref%29))
  ;[1 1 1] ChoppingEvent
  (Class|BPIInteractable|ChopChop(Message) OtherActor (Utilities|GetDamagefromGI)))

(event OnComponentBeginOverlap(Sphere)
  (params (OverlappedComponent :type Primitive%20Component%20Object%20Reference) (OtherActor :type Actor%20Object%20Reference) (OtherComp :type Primitive%20Component%20Object%20Reference) (OtherBodyIndex :type Integer) (bFromSweep :type Boolean) (SweepResult :type Hit%20Result%20Structure%20%28by%20ref%29))
  ;[1 1 1] ArrayingThingsToChop
  (if (Utilities|DoesObjectImplementInterface OtherActor "/Game/Lumberman/Interfaces/BPI_Interactable.BPI_Interactable_C")
    (Utilities|Array|AddUnique (Variables|Default|GetThingsToChopArray) OtherActor)))

(event OnComponentEndOverlap(Sphere)
  (params (OverlappedComponent :type Primitive%20Component%20Object%20Reference) (OtherActor :type Actor%20Object%20Reference) (OtherComp :type Primitive%20Component%20Object%20Reference) (OtherBodyIndex :type Integer))
  ;[1 1 1] ArrayingThingsToChop
  (if (Utilities|DoesObjectImplementInterface OtherActor "/Game/Lumberman/Interfaces/BPI_Interactable.BPI_Interactable_C")
    (Utilities|Array|RemoveItem (Variables|Default|GetThingsToChopArray) OtherActor)))

(event Custom|CanChopChop?
  ;[1 1 1] ChoppingEvent
  (if (Utilities|Array|IsEmpty (Variables|Default|GetThingsToChopArray))
    (Collision|SetCollisionEnabled (Variables|Default|Getr) "NoCollision")
    (else
      (Collision|SetCollisionEnabled (Variables|Default|Getr) "QueryOnly")
      (Animation|PlayAnimMontage "/Game/Lumberman/Assets/Animations/PlayerCharacter/360SwingMontage.360SwingMontage" 1.0 "None"))))

(event EventBeginPlay
  ;[1 1 1] InitializeHP,GI,Chopping
  (Utilities|FlowControl|Sequence
    (:then_1
      (Utilities|Time|SetTimerbyEvent (delegate Custom|CanChopChop?) 1.0 true true 1.0))
    (:then_2
      (CallFunction|ResetHP))))

(event EventTakeDamage
  (params (Damage :type Float%20%28double-precision%29))
  (Default|TakeDamage (CallFunction|GetGi) Damage))

(event Input|AxisEvents|InputAxisMoveForward
  (params (AxisValue :type Float%20%28single-precision%29))
  ;[1 1 1] Movement
  (Pawn|Input|AddMovementInput (Math|Vector|MakeVector AxisValue 0.0 0.0) 1.0 false))

(event Input|AxisEvents|InputAxisMoveRight
  (params (AxisValue :type Float%20%28single-precision%29))
  ;[1 1 1] Movement
  (Pawn|Input|AddMovementInput (Math|Vector|MakeVector 0.0 AxisValue 0.0) 1.0 false))

(fn ConstructionScript
  (Transformation|AttachComponentToComponent (Variables|Default|GetAxe) (Variables|Character|GetMesh) "RightHandSocket" "KeepRelative" "KeepRelative" "KeepRelative" false))

(fn ResetHP
  (bind _asgi (CallFunction|GetGi))
  (Default|SetPlayerStats _asgi (LocalVariables|GetNewLocalVar) (.Value (Utilities|Map|Find (Default|GetPlayerStats _asgi) "NewEnumerator1"))))
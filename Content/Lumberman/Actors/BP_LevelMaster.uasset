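; BP_LevelMaster sets up a dungeon level from the player's saved progress.
; On BeginPlay it reads the dungeon level from the game instance's progress map and loads that row from LevelDataTable.
; It then passes the level number to all BPI_Gauntlet actors and spawns a BP_Tree at each tree location in the row.
; A separate OpenGates event opens every BP_LevelGate in the level.
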(event EventBeginPlay
  (Utilities|FlowControl|Sequence
    (:then_0
      ;[1 1 1] MoveToConstructionScript
      (bind _output_get (Variables|Default|SetDungeonLevel (.Value (Utilities|Map|Find (Default|GetPlayerProgress (CallFunction|GetGi)) "NewEnumerator6"))))
      (bind _returnvalue (Utilities|GetDataTableRow "/Game/Lumberman/Architecture/LevelDataTable.LevelDataTable" (Utilities|String|StringToName (Utilities|String|ToString(Integer) _output_get)))
        (:then
          (Variables|Default|SetLevelData _returnvalue))
        (:RowNotFound
          (Development|PrintString (Utilities|String|Append "RowN N not found:" (Utilities|String|ToString(Integer) _output_get))))))
    (:then_1
      (bind _outactors (Actor|GetAllActorswithInterface "/Game/Lumberman/Interfaces/BPI_Gauntlet.BPI_Gauntlet_C"))
      (for _array_element _outactors
        (Class|BPIGauntlet|GetDungeonLevel(Message) _array_element (Variables|Default|GetDungeonLevel))))
    (:then_2
      ;[1 1 1] TreeSpawning
      (for _array_element_2 (.treelocations (Variables|Default|GetLevelData))
        (Game|SpawnActorfromClass "/Game/Lumberman/Actors/BP_Tree.BP_Tree_C" (Math|Conversions|ToTransform(Vector) _array_element_2) "AdjustIfPossibleButAlwaysSpawn" "MultiplyWithRoot" 0 0)))))

(event EventOpenGates
  (bind _outactors (Actor|GetAllActorsOfClass "/Game/Lumberman/Actors/BP_LevelGate.BP_LevelGate_C"))
  (for _array_element _outactors
    (Default|OpenGates _array_element)))

(fn ConstructionScript)
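; BP_LevelGate is a level exit gate that moves the player to another map when they touch it after it has been opened.
; A Gate node blocks the player's collision overlap until OpenGates opens it.
; A return gate, marked by a different cube material at BeginPlay, loads BaseLevel.
; Other gates save DungeonLevel plus one as player progress through the game instance, then load GauntletLevel.
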(event OnComponentBeginOverlap(Collision)
  (params (OverlappedComponent :type Primitive%20Component%20Object%20Reference) (OtherActor :type Actor%20Object%20Reference) (OtherComp :type Primitive%20Component%20Object%20Reference) (OtherBodyIndex :type Integer) (bFromSweep :type Boolean) (SweepResult :type Hit%20Result%20Structure%20%28by%20ref%29))
  (if (== OtherActor (Game|Player|GetPlayerPawn 0))
    (Utilities|FlowControl|Gate (Variables|Default|GetStart%20Closed)
      (:Exit
        (if (Variables|Default|GetbReturnGate?)
          (Game|OpenLevel(byName) (Variables|Default|GetBaseLevel))
          (else
            (Default|AddPlayerProgress (CallFunction|GetGi) (Variables|Default|GetKey) (+ (Variables|Default|GetDungeon%20Level) 1))
            (Game|OpenLevel(byName) (Variables|Default|GetGauntletLevel))))))))

(event EventBeginPlay
  (if (Variables|Default|GetbReturnGate?)
    (Rendering|Material|SetMaterial (Variables|Default|GetCube) 0 "/Engine/MapTemplates/Materials/BasicAsset02.BasicAsset02")
    (Rendering|Material|SetMaterial (Variables|Default|GetCube1) 0 "/Engine/MapTemplates/Materials/BasicAsset02.BasicAsset02")))

(event EventGetDungeonLevel
  (params (DungeonLevel :type Integer))
  (Variables|Default|SetDungeon%20Level DungeonLevel))

(event EventOpenGates
  (Utilities|FlowControl|Gate (Variables|Default|GetStart%20Closed)) ; enters at Open
)

(fn ConstructionScript)
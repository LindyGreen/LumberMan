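; BP_Well is a building actor in the Lumberman game that provides a health upgrade to the player.
; UpgradePlayerStats reads the building's progress level from the game instance, scales it by a fixed bonus, adds it to a stored stat, and writes both max and current HP.
; The collision overlap only checks for the player character with no action attached, and nothing in this Blueprint calls the upgrade function.
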(event OnComponentBeginOverlap(Collision)
  (params (OverlappedComponent :type Primitive%20Component%20Object%20Reference) (OtherActor :type Actor%20Object%20Reference) (OtherComp :type Primitive%20Component%20Object%20Reference) (OtherBodyIndex :type Integer) (bFromSweep :type Boolean) (SweepResult :type Hit%20Result%20Structure%20%28by%20ref%29))
  (if (== OtherActor (Game|GetPlayerCharacter 0))
    _))

(event EventBeginPlay
  (|CallParentFunction) ; This node is disabled and will not be called.\nDrag off pins to build functionality.
)

(event Collision|EventActorBeginOverlap
  (params (OtherActor :type Actor%20Object%20Reference)))

(event EventTick
  (params (DeltaSeconds :type Float%20%28single-precision%29)))

(fn ConstructionScript
  (|CallParentFunction))

(fn UpgradePlayerStats
  (bind _asgi (CallFunction|GetGi))
  (bind _buildingkey (Variables|Default|GetBuildingKey))
  (bind _playerstats (Default|GetPlayerStats _asgi))
  (bind _playerprogress (Default|GetPlayerProgress _asgi))
  (bind _value (Utilities|Map|Find _playerprogress _buildingkey))
  (bind _value_2 (Utilities|Map|Find _playerstats "NewEnumerator1"))
  (bind _returnvalue (* _value 20))
  (bind _returnvalue_2 (+ _returnvalue _value_2))
  (Default|SetPlayerStats _asgi (LocalVariables|GetMaxHP_Enum) _returnvalue_2)
  (Default|SetPlayerStats _asgi (LocalVariables|GetHP_Enum) _returnvalue_2))
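; Base building actor for the Lumberman game that the player upgrades with score, with its level saved in game instance progress under BuildingKey.
; The level indexes both the mesh and upgrade cost arrays, setting the look on BeginPlay and after upgrades.
; Upgrade gates on score, charges the cost, increments the level, refreshes the widget and calls UpgradePlayerStats, left empty for child overrides.
; A collision overlap shows the widget only while the player is near.
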(event OnComponentBeginOverlap(Collision)
  (params (OverlappedComponent :type Primitive%20Component%20Object%20Reference) (OtherActor :type Actor%20Object%20Reference) (OtherComp :type Primitive%20Component%20Object%20Reference) (OtherBodyIndex :type Integer) (bFromSweep :type Boolean) (SweepResult :type Hit%20Result%20Structure%20%28by%20ref%29))
  (if (== OtherActor (Game|GetPlayerCharacter 0))
    (Rendering|SetVisibility (Variables|Default|GetWidget) true false)))

(event OnComponentEndOverlap(Collision)
  (params (OverlappedComponent :type Primitive%20Component%20Object%20Reference) (OtherActor :type Actor%20Object%20Reference) (OtherComp :type Primitive%20Component%20Object%20Reference) (OtherBodyIndex :type Integer))
  (if (== OtherActor (Game|GetPlayerCharacter 0))
    (Rendering|SetVisibility (Variables|Default|GetWidget) false false)))

(event EventBeginPlay
  (bind _widget (Variables|Default|GetWidget))
  (bind _returnvalue (UserInterface|GetWidget _widget))
  (CallFunction|GetGiInitializeMesh (Variables|Default|GetBuildingKey))
  (Class|BPIUI|GetOwnerBuilding(Message) _returnvalue self)
  (Class|BPIUI|GetUpgradeCost(Message) _returnvalue (Utilities|Array|Get(acopy) (Variables|Default|GetUpgradeCost) (.Value (Utilities|Map|Find (Default|GetPlayerProgress (CallFunction|GetGi)) (Variables|Default|GetBuildingKey))))))

(event EventUpgrade
  (bind _buildingkey (Variables|Default|GetBuildingKey))
  (Utilities|CanUpgradeBuilding? _buildingkey)
  (CallFunction|UpgradeBuildingMesh _buildingkey)
  (Class|BPIUI|GetUpgradeCost(Message) (UserInterface|GetWidget (Variables|Default|GetWidget)) (Utilities|Array|Get(acopy) (Variables|Default|GetUpgradeCost) (.Value (Utilities|Map|Find (Default|GetPlayerProgress (CallFunction|GetGi)) (Variables|Default|GetBuildingKey)))))
  (CallFunction|UpgradePlayerStats) ; its empty as I will be overwriting it in all buildings
)

(fn ConstructionScript)

(fn UpgradeBuildingMesh
  (params (KeyToUpgdare :type E_Progress%20Enum%20%28by%20ref%29 :default "NewEnumerator0"))
  (bind _asgi (CallFunction|GetGi))
  (bind _result (Math|Integer|IncrementInt (.Value (Utilities|Map|Find (Default|GetPlayerProgress _asgi) KeyToUpgdare)))
    (:%20%20
      (Default|AddPlayerProgress _asgi KeyToUpgdare _result)
      (Components|StaticMesh|SetStaticMesh (Variables|Default|GetStaticMesh) (Utilities|Array|Get(acopy) (Variables|Default|GetStaticMeshes) _result)))))

(fn ActivateBuilding)

(fn GetGiInitializeMesh
  (params (Key :type E_Progress%20Enum%20%28by%20ref%29 :default "NewEnumerator0"))
  (Components|StaticMesh|SetStaticMesh (Variables|Default|GetStaticMesh) (Utilities|Array|Get(acopy) (Variables|Default|GetStaticMeshes) (.Value (Utilities|Map|Find (Default|GetPlayerProgress (CallFunction|GetGi)) Key)))))

(fn UpgradePlayerStats)
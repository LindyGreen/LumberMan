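; Choppable tree actor for the Lumberman game that awards score as it is harvested segment by segment.
; The construction script randomizes width and height, scales the collision, and builds a stack of static mesh segments.
; ChopChop, throttled by a half-second gate, or a debug key triggers HarvestTree, which removes segments bottom-up and sends width-based score to the GameInstance.
; The actor destroys itself after the final segment, and WhatTypeAreYou reports its type enum.
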(event Custom|HarvestTree
  (bind _treesegmentsarray (Variables|Default|GetTreeSegmentsArray))
  (bind _choppingprogress (Variables|Default|GetChoppingProgress))
  (bind _output (Utilities|Array|Get(acopy) _treesegmentsarray _choppingprogress))
  (Utilities|IsValid _output
    (:Is%20Valid
      (Components|DestroyComponent _output)
      (Class|BPIGI|ChangeScore(Message) (Game|GetGameInstance) (Math|Float|Truncate (Variables|TreeSize|GetTreeWidth)))
      (bind _result (Math|Integer|IncrementInt (Variables|Default|GetChoppingProgress))
        (:%20%20
          (if (> _result (Variables|Default|GetInitialTreeHight))
            (Utilities|FlowControl|Delay 1.0)
            (Actor|DestroyActor)))))))

(event EventBeginPlay
  (Input|EnableInput (Game|GetPlayerController 0)))

(event EventChopChop
  (params (Damage :type Float%20%28double-precision%29))
  (Utilities|FlowControl|Gate false :!label _label
    (:Exit
      (CallFunction|HarvestTree)
      (Utilities|FlowControl|Sequence
        (:then_0
          (goto _label Close))
        (:then_1
          (Utilities|FlowControl|Delay 0.5)
          (goto _label Open))))))

(event Input|KeyboardEvents|DebugKey1
  (params (Key :type Key%20Structure :default "None") (ActionValue :type Input%20Action%20Value%20Structure))
  (:Pressed
    (CallFunction|HarvestTree)))

(fn ConstructionScript
  (bind _returnvalue (|({57B3B83A-43BE-690A-2832-80BAC8AFAED1}/5)))
  (bind _output_get (Variables|TreeSize|SetTreeWidth (Math|Conversions|ToFloat(Integer) (Math|Random|RandomIntegerinRange (Variables|TreeSize|GetMin%20TreeWidth) (Variables|TreeSize|GetMaxTreeWidth)))))
  (Transformation|SetRelativeScale3D (Variables|Default|GetCollision) (Math|Vector|MakeVector _output_get _output_get 2e+02))
  (bind _output_get_2 (Variables|Default|SetInitialTreeHight (Math|Random|RandomIntegerinRange (Variables|TreeSize|GetMinTreeHeight) (Variables|TreeSize|GetMaxTreeHeight))))
  (for _index (range 0 _output_get_2)
    (bind _returnvalue_2 (AddComponent|AddStaticMeshComponent false (Math|Transform|MakeTransform (Math|Vector|MakeVector 0.0 0.0 (|((N*100)+50) (Math|Conversions|ToFloat(Integer) _index))) "0, 0, 0" (Math|Vector|MakeVector _returnvalue _returnvalue 1.0))))
    (Utilities|Array|AddUnique (Variables|Default|GetTreeSegmentsArray) _returnvalue_2))
  (Development|PrintString "Construction SCript Succeeded"))

(fn WhatTypeAreYou
  (return (Variables|Default|GetEnumType)))